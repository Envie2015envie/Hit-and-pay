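; BP_CashTaker is a clickable actor that triggers the first-person character's money count when a product is selected.
; On BeginPlay it casts and caches the player character as BP_FirstPersonCharacter.
; Clicking its CashTaker component checks that the character's SelectedProduct is valid, then spawns a half-scale hit particle at the actor and calls CountOfMoney on the character.
; Debug strings print on click and on success.
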(event OnClicked(CashTaker)
  (params (TouchedComponent :type Primitive%20Component%20Object%20Reference) (ButtonPressed :type Key%20Structure :default "None"))
  (Development|PrintString "i tuched")
  (Utilities|IsValid (Variables|/Game/FirstPerson/Blueprints/BP_FirstPersonCharacter.BP_FirstPersonCharacter_C|GetSelected%20Product (Variables|Default|GetAs%20BP%20First%20Person%20Character))
    (:Is%20Valid
      (Effects|SpawnEmitteratLocation "/Game/LowPolyVFX/Particles/P_Ems_Hit_02.P_Ems_Hit_02" (Transformation|GetActorLocation) "0, 0, 0" "0.500000,0.500000,0.500000")
      (Development|PrintString "i work")
      (Default|CountOfMoney (Variables|Default|GetAs%20BP%20First%20Person%20Character)))))

(event EventBeginPlay
  (bind _asbp_first_person_character (Utilities|Casting|CastToBP_FirstPersonCharacter (Game|GetPlayerCharacter 0)))
  (Variables|Default|SetAs%20BP%20First%20Person%20Character _asbp_first_person_character))

(fn ConstructionScript)