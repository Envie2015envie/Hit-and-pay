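; BP_Door is a door Blueprint that swings open when its OpenDoor event is called, then closes itself.
; A timeline drives the Door component's relative pitch, and on finishing waits briefly before reversing.
; A DoOnce, reset on each OpenDoor call, stops the reverse pass from retriggering the cycle.
; BeginPlay enables click events on the player controller, but the Door's OnClicked handler is empty.
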(event OnClicked(Door)
  (params (TouchedComponent :type Primitive%20Component%20Object%20Reference) (ButtonPressed :type Key%20Structure :default "None")))

(event Custom|Open%20Door
  (Utilities|FlowControl|Sequence
    (:then_0
      (bind _doortime (Timeline|Timeline_0 PlayFromStart)
        (:Update
          (Transformation|SetRelativeRotation (Variables|Default|GetDoor) (Math|Rotator|MakeRotator 0.0 (* _doortime 1e+02) 0.0) false false))
        (:Finished
          (Utilities|FlowControl|DoOnce false :!label _label
            (:Completed
              (Utilities|FlowControl|Delay 1.0)
              (Timeline|Timeline_0 ReverseFromEnd))))))
    (:then_1
      (goto _label Reset))))

(event EventBeginPlay
  (Utilities|FlowControl|Sequence
    (:then_0
      (Variables|/Script/Engine.PlayerController|SetbEnableClickEvents (Game|GetPlayerController 0) true))))

(fn ConstructionScript)