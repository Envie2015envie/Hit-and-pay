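; BP_MainProduct is a product actor that destroys BP_Product actors overlapping its Collision component.
; On overlap it spawns a small explosion emitter at its own location, then destroys the other product after a short delay.
; A Displacement event subtracts WeightOfProduct values and tests the result in sequenced branches, all empty.
; A MainProduct world-offset call is left unconnected, so no movement happens here.
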(event OnComponentBeginOverlap(collision)
  (params (OverlappedComponent :type Primitive%20Component%20Object%20Reference) (OtherActor :type Actor%20Object%20Reference) (OtherComp :type Primitive%20Component%20Object%20Reference) (OtherBodyIndex :type Integer) (bFromSweep :type Boolean) (SweepResult :type Hit%20Result%20Structure%20%28by%20ref%29))
  (bind _asbp_product (Utilities|Casting|CastToBP_Product OtherActor))
  (Effects|SpawnEmitteratLocation "/Game/LowPolyVFX/Particles/P_Ems_Explosion_04.P_Ems_Explosion_04" (Transformation|GetActorLocation) "0, 0, 0" "0.300000,0.300000,0.300000")
  (Utilities|FlowControl|Delay 0.5)
  (Utilities|IsValid _asbp_product
    (:Is%20Valid
      (Actor|DestroyActor _asbp_product))))

(event Custom|Displacement
  (bind _output_get (Variables|Default|SetWeight%20of%20product (Variables|Default|GetWeight%20of%20product)))
  (bind _output_get_2 (Variables|Default|SetWeight%20of%20product (- _output_get (Variables|Default|GetWeight%20of%20product))))
  (Utilities|FlowControl|Sequence
    (:then_0
      (if (< _output_get_2 0)
        _))
    (:then_1
      (if (== _output_get_2 0)
        _))
    (:then_2
      (if (== _output_get_2 1)
        _))
    (:then_3
      (if (== _output_get_2 2)
        _))
    (:then_4
      (if (== _output_get_2 3)
        _))
    (:then_5
      (if (== _output_get_2 4)
        _))))

(event EventBeginPlay)

(event Collision|EventActorBeginOverlap
  (params (OtherActor :type Actor%20Object%20Reference)))

(event EventTick
  (params (DeltaSeconds :type Float%20%28single-precision%29)))

(fn ConstructionScript)