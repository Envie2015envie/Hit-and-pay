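; BP_Product is a clickable product with a price and configurable mesh, apparently an item in a spiral vending machine.
; BeginPlay caches the first-person character and cash taker; clicking registers the product as the character's SelectedProduct.
; Falling enables mesh physics, clears that selection and triggers the linked BP_Spiral, while Activ unhides the mesh.
; Click-event enabling and money-count calls are unwired, and debug prints remain.
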(event OnClicked(Product)
  (params (TouchedComponent :type Primitive%20Component%20Object%20Reference) (ButtonPressed :type Key%20Structure :default "None"))
  (Variables|/Game/FirstPerson/Blueprints/BP_FirstPersonCharacter.BP_FirstPersonCharacter_C|SetSelected%20Product (Variables|Default|GetCharacter%20ref) self)
  (Development|PrintString "Hello"))

(event Custom|Falling
  (Development|PrintString "aaaaa")
  (Physics|SetSimulatePhysics (Variables|Default|GetProduct) true)
  (Variables|/Game/FirstPerson/Blueprints/BP_FirstPersonCharacter.BP_FirstPersonCharacter_C|SetSelected%20Product (Variables|Default|GetCharacter%20ref) 0)
  (bind _asbp_spiral (Utilities|Casting|CastToBP_Spiral (Variables|Default|GetSpiral)))
  (bind _output_get (Variables|Default|SetAs%20BP%20Spiral _asbp_spiral))
  (Default|ActivSpiral _output_get))

(event Custom|Activ
  (Development|SetHiddeninGame (Variables|Default|GetProduct) false false))

(event EventBeginPlay
  (Variables|Default|SetPrice (Variables|Default|GetPrice))
  (bind _asbp_first_person_character (Utilities|Casting|CastToBP_FirstPersonCharacter (Game|GetPlayerCharacter 0)))
  (Variables|Default|SetCharacter%20ref _asbp_first_person_character)
  (bind _returnvalue (Actor|GetActorOfClass "/Game/Blueprints/BP_CashTaker.BP_CashTaker_C"))
  (Variables|Default|SetCash%20Taker%20Ref _returnvalue))

(fn ConstructionScript
  (Components|StaticMesh|SetStaticMesh (Variables|Default|GetProduct) (Variables|Default|GetMesh)))