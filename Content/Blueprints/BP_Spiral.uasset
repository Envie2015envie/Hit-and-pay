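; BP_Spiral is a clickable spiral that dispenses a product, apparently for a vending-style machine.
; Its construction script assigns the product mesh from the NewMesh variable.
; Clicking Spiral plays the ProductMov timeline to slide the mesh along its local X axis, then hides it and calls Activ on BPProduct.
; The Activspiral event only checks a BP_Spiral reference for validity and takes no further action.
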(event OnClicked(Spiral)
  (params (TouchedComponent :type Primitive%20Component%20Object%20Reference) (ButtonPressed :type Key%20Structure :default "None"))
  (bind _alpha (Timeline|ProductMov PlayFromStart)
    (:Update
      (Transformation|SetRelativeLocation (Variables|Default|GetMesh) (Math|Vector|MakeVector (Math|Float|Lerp 0.0 -43.0 _alpha) 0.0 -3.346891) false false))
    (:Finished
      (Rendering|SetVisibility (Variables|Default|GetMesh) false false)
      (Default|Activ (Variables|Default|GetBP%20Product)))))

(event Custom|Activ%20spiral
  (Utilities|IsValid "BP_Spiral"))

(event EventBeginPlay)

(fn ConstructionScript
  (Components|StaticMesh|SetStaticMesh (Variables|Default|GetMesh) (Variables|Default|GetNew%20Mesh)))