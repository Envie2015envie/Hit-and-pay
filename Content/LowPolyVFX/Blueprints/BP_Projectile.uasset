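; BP_Projectile is a simple projectile actor from the LowPolyVFX folder that moves itself along world X.
; On BeginPlay a timeline runs, and each update offsets the root by the Wave variable with a swept, teleporting move.
; Wave is set from the scaled timeline track only when the timeline finishes, so the movement uses its prior value.
; Tick and overlap do nothing, and an unused sine calculation remains.
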(event EventBeginPlay
  (bind _wave (Timeline|Timeline_0 Play)
    (:Update
      (Transformation|SetWorldLocation (Variables|Default|GetDefaultSceneRoot) (+ (Transformation|GetWorldLocation (Variables|Default|GetDefaultSceneRoot)) (Math|Vector|MakeVector (Variables|Default|Getwave) 0.0 0.0)) true true))
    (:finish
      (Variables|Default|Setwave (* _wave 5.0)))))

(event Collision|EventActorBeginOverlap
  (params (OtherActor :type Actor%20Object%20Reference)))

(event EventTick
  (params (DeltaSeconds :type Float%20%28single-precision%29)))

(fn ConstructionScript)